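; Game State for a multiplayer match that tracks connected players and runs the match's timed phases.
; Players are counted against the Game Instance's limit, with overflow triggering a session destroy and main-menu load.
; One-second looping timers count down to match start, match end and session shutdown, calling the Game Mode or preparing controllers for server travel.
; Each tick sends every player controller the countdown matching the current MatchState.
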(event Custom|RemovePlayer
  (params (ExitingController :type Controller%20Object%20Reference))
  ;[1 1 1] Удалить игрока из Game State
  (Variables|Default|SetCurrentPlayers (- (Variables|Default|GetCurrentPlayers) 1))
  (bind _asgameplay_player_controller (Utilities|Casting|CastToGameplayPlayerController ExitingController))
  (Utilities|Array|RemoveItem (Variables|Default|GetPlayerControllers) _asgameplay_player_controller))

(event Custom|AddPlayer
  (params (PlayerController :type Player%20Controller%20Object%20Reference))
  ;[1 1 1] Добавляет игрока в Game State
  (bind _asmultiplayer_template_game_instance (Utilities|Casting|CastToMultiplayerTemplateGameInstance (Game|GetGameInstance)))
  (if (< (Variables|Default|GetCurrentPlayers) (Variables|/Game/MultiplayerTemplate/Blueprints/AllLevels/MultiplayerTemplateGameInstance.MultiplayerTemplateGameInstance_C|GetMaxPlayers _asmultiplayer_template_game_instance))
    (Variables|Default|SetCurrentPlayers (+ (Variables|Default|GetCurrentPlayers) 1))
    (bind _asgameplay_player_controller (Utilities|Casting|CastToGameplayPlayerController PlayerController))
    (Utilities|Array|Add (Variables|Default|GetPlayerControllers) _asgameplay_player_controller)
    (else
      (|DestroySession PlayerController
        (:OnSuccess
          (Game|OpenLevel(byName) "MainMenuMap"))))))

(event Custom|TimerCheckME
  (bind _matchtime (Variables|Default|GetMatchTime))
  ;[1 0 0] Обратный отсчет до конца матча
  (Math|Integer|DecrementInt _matchtime
    (:%20%20
      (if (< _matchtime 0)
        (Utilities|Time|ClearandInvalidateTimerbyHandle (stale Custom|CustomEvent_0 _returnvalue))
        (bind _asgameplay_game_mode (Utilities|Casting|CastToGameplayGameMode (Game|GetGameMode)))
        (Class|GameMode|EndMatch _asgameplay_game_mode)
        (else
          (CallFunction|TellClienttoCountdown))))))

(event Custom|CountdownTimerToMatchEnd
  ;[1 0 0] Обратный отсчет до конца матча
)

(event Custom|DestroySession
  ;[1 1 1] Закрыть сессию
  (for _array_element (Variables|Default|GetPlayerControllers)
    (Default|PrepareforServerTravel _array_element)))

(event Custom|CountdownToDestroySession
  ;[1 1 1] Обратный отсчет до конца сеесси
  (bind _returnvalue (Utilities|Time|SetTimerbyEvent (delegate Custom|TimerCheckDS) 1.0 true)))

(event Custom|TimerCheckSM
  (bind _timebeforestartmatch (Variables|Default|GetTimeBeforeStartMatch))
  ;[1 1 1] Обратный отсчет до начала матча
  (Math|Integer|DecrementInt _timebeforestartmatch
    (:%20%20
      (if (< _timebeforestartmatch 0)
        (Utilities|Time|ClearandInvalidateTimerbyHandle (stale Custom|CountdownTimerToStartMatch _returnvalue))
        (bind _asgameplay_game_mode (Utilities|Casting|CastToGameplayGameMode (Game|GetGameMode)))
        (Class|GameMode|StartMatch _asgameplay_game_mode)
        (else
          (CallFunction|TellClienttoCountdown))))))

(event Custom|TimerCheckDS
  (bind _timeafterendmatch (Variables|Default|GetTimeAfterEndMatch))
  ;[1 1 1] Обратный отсчет до конца сеесси
  (Math|Integer|DecrementInt _timeafterendmatch
    (:%20%20
      (if (< _timeafterendmatch 0)
        (Utilities|Time|ClearandInvalidateTimerbyHandle (stale Custom|CountdownToDestroySession _returnvalue))
        (CallFunction|DestroySession)
        (else
          (CallFunction|TellClienttoCountdown))))))

(event Custom|CountdownTimerToStartMatch
  ;[1 1 1] Обратный отсчет до начала матча
  (bind _returnvalue (Utilities|Time|SetTimerbyEvent (delegate Custom|TimerCheckSM) 1.0 true)))

(event Custom|CustomEvent_0
  ;[1 0 0] Обратный отсчет до конца матча
  (bind _returnvalue (Utilities|Time|SetTimerbyEvent (delegate Custom|TimerCheckME) 1.0 true)))

(event Custom|TellClientToCountdown
  ;[1 1 1] Номера Таймера появления
  (for _array_element (Variables|Default|GetPlayerControllers)
    (switch name (Variables|Default|GetMatchState)
      (:WaitingToStart
        (Default|SpawnCountdownTimeStart _array_element (Variables|Default|GetTimeBeforeStartMatch)))
      (:InProgress
        (Default|SpawnCountdownTimeGameOver _array_element (Variables|Default|GetMatchTime)))
      (:WaitingPostMatch
        (Default|SpawnCountdownTimeByeBye _array_element (Variables|Default|GetTimeAfterEndMatch))))))

(event EventBeginPlay
  ;[1 1 1] Инициализировать состояние Game State
  (Networking|SwitchHasAuthority
    (:Authority
      (bind _asmultiplayer_template_game_instance (Utilities|Casting|CastToMultiplayerTemplateGameInstance (Game|GetGameInstance)))
      (Variables|Default|SetMaxPlayers (Variables|/Game/MultiplayerTemplate/Blueprints/AllLevels/MultiplayerTemplateGameInstance.MultiplayerTemplateGameInstance_C|GetMaxPlayers _asmultiplayer_template_game_instance))
      (CallFunction|CountdownTimertoStartMatch))))

(fn ConstructionScript)