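; LobbyPlayerController is the multiplayer lobby player controller that drives each player's lobby UI.
; Initial setup clears existing widgets, shows the lobby menu and enables the mouse cursor.
; Further events pass player-list updates to that menu and spawn a start countdown widget with a given number of seconds.
; Before server travel, it asks the game instance to show the loading screen.
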(event Custom|ShowLobbyMenu
  ;[1 1 1] Показать меню лобби
  (Viewport|RemoveAllWidgets)
  (bind _returnvalue (UserInterface|CreateWidget "/Game/MultiplayerTemplate/Blueprints/Lobby/WBP_LobbyMenu.WBP_LobbyMenu_C" self))
  (bind _output_get (Variables|Default|SetWBP_LobbyMenu _returnvalue))
  (UserInterface|Viewport|AddtoViewport _output_get 0)
  (Variables|Default|SetbShowMouseCursor true))

(event Custom|UpdatePlayerList
  (params (UniqueNetIDs :type Array%20of%20Strings) (PlayerInfos :type Array%20of%20Player%20Info%20Structures))
  (bind _wbp_lobbymenu (Variables|Default|GetWBP_LobbyMenu))
  ;[1 1 1] Обновить список игроков
  (Utilities|IsValid _wbp_lobbymenu
    (:Is%20Valid
      (Default|UpdatePlayerList _wbp_lobbymenu UniqueNetIDs PlayerInfos))))

(event Custom|PrepareForServerTravel
  ;[1 1 1] Загрузочный экран
  (bind _asmultiplayer_template_game_instance (Utilities|Casting|CastToMultiplayerTemplateGameInstance (Game|GetGameInstance)))
  (Default|ShowLoadingScreen _asmultiplayer_template_game_instance))

(event Custom|InitialSetup
  ;[1 1 1] Начальная настройка
  (CallFunction|ShowLobbyMenu))

(event Custom|SpawnCountdownTime
  (params (Seconds :type Integer))
  ;[1 1 1] Показать таймер обратного отсчета
  (bind _returnvalue (UserInterface|CreateWidget "/Game/MultiplayerTemplate/Blueprints/AllLevels/WBP_Countdown_Time_Start.WBP_Countdown_Time_Start_C" 0 Seconds))
  (UserInterface|Viewport|AddtoViewport _returnvalue 0))

(fn ConstructionScript)